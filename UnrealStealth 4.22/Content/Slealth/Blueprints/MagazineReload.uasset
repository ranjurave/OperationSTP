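; MagazineReload is a spinning ammo pickup that refills the player's bullets.
; On overlap with PlayerCharBP, only when its bullet count is empty, it sets the count to 10, spawns a particle effect and destroys itself.
; Tick advances the yaw by a fixed step each frame, so spin speed depends on frame rate.
; An unfinished, disconnected branch sketches partial refills drawn from a magazine's own bullet reserve.
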(event `self.ReceiveBeginPlay`
  (bind _asplayer_char_bp (cast `/Game/Slealth/Blueprints/PlayerCharBP` (`GameplayStatics.GetPlayerCharacter` 0)))
  (set `self.PlayerChar` _asplayer_char_bp))

(event `self.ReceiveActorBeginOverlap`
  (params (OtherActor :type "Actor Object Reference"))
  (cast `/Game/Slealth/Blueprints/PlayerCharBP` OtherActor)
  (if (<= (`/Game/Slealth/Blueprints/PlayerCharBP.BulletCount` (`self.PlayerChar`)) 0)
    (set `/Game/Slealth/Blueprints/PlayerCharBP.BulletCount` 10 (`self.PlayerChar`))
    (`GameplayStatics.SpawnEmitterAtLocation` "/Game/Slealth/Particles/MagazineParticles.MagazineParticles" (`self.K2_GetActorLocation`) (struct) (0.8 0.8 0.8))
    (`self.K2_DestroyActor`)))

(event `self.ReceiveTick`
  (params (DeltaSeconds :type "Float (single-precision)"))
  (bind _output_get (set `self.rotation` (.yaw (`self.K2_GetActorRotation`))))
  (`self.K2_SetActorRotation` (`KismetMathLibrary.MakeRotator` 0.0 0.0 (+ _output_get 1.0))))

(fn `UserConstructionScript`)