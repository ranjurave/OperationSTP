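; Enemy character Blueprint that shoots bullets and dies after taking a set number of bullet hits.
; Each Bullet hit decrements BulletHit, playing a hit montage through a resettable DoOnce while hits remain.
; At zero, a second DoOnce plays the death montage, then destroys the actor after a short delay.
; ShootPlayer sets IsFiring, spawns a Bullet offset from SphereTPS along the capsule's rotation, and emits muzzle-fire particles.
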(event `ResetDo`
  ;[1 1 1] Bullet hit
  (goto _label :!via `Reset`))

(event `self.ReceiveHit`
  (params (MyComp :type "PrimitiveComponent Object Reference") (Other :type "Actor Object Reference") (OtherComp :type "PrimitiveComponent Object Reference") (bSelfMoved :type Boolean) (HitLocation :type "Vector Structure") (HitNormal :type "Vector Structure") (NormalImpulse :type "Vector Structure") (Hit :type "HitResult Structure (by ref)"))
  ;[1 1 1] Bullet hit
  (cast `/Game/Slealth/Blueprints/Bullet` Other)
  (bind _result (`/Engine/EditorBlueprintResources/StandardMacros.DecrementInt` (`self.BulletHit`))
    (:`  `
      (set `self.BulletHit` _result)
      (if (> (`self.BulletHit`) 0)
        (`/Engine/EditorBlueprintResources/StandardMacros.DoOnce` false :!label _label
          (:`Completed`
            (`AnimInstance.Montage_Play` (`SkeletalMeshComponent.GetAnimInstance` (`self.Mesh`)) "/Game/Slealth/Animations/EnemyAnimation/HitEnemyMontage.HitEnemyMontage" 1.0 "MontageLength" 0.0 true)
            (`self.ResetDo`)))
        (else
          (`/Engine/EditorBlueprintResources/StandardMacros.DoOnce` false
            (:`Completed`
              (`AnimInstance.Montage_Play` (`SkeletalMeshComponent.GetAnimInstance` (`self.Mesh`)) "/Game/Slealth/Animations/EnemyAnimation/DeathEnemyMontage.DeathEnemyMontage" 1.0 "MontageLength" 0.0 true)
              (`KismetSystemLibrary.Delay` 1.6)
              (`self.K2_DestroyActor`))))))))

(event `ShootPlayer`
  (bind _returnvalue (`SceneComponent.K2_GetComponentRotation` (`self.CapsuleComponent`)))
  ;[1 1 1] Third person shooting
  (set `self.IsFiring` true)
  (`|SpawnActorFromClass` "/Game/Slealth/Blueprints/Bullet.Bullet_C" (`KismetMathLibrary.MakeTransform` (+ (`SceneComponent.K2_GetComponentLocation` (`self.SphereTPS`)) (`KismetMathLibrary.GreaterGreater_VectorRotator` (`self.GunOffsetTPS`) _returnvalue)) _returnvalue) "Undefined" "OverrideRootScale" null null)
  (`GameplayStatics.SpawnEmitterAtLocation` "/Game/Slealth/Particles/GunFireParticles.GunFireParticles" (`SceneComponent.K2_GetComponentLocation` (`self.SphereTPS`)) (struct) (0.2 0.2 0.2)))

(fn `UserConstructionScript`)