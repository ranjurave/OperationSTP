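; Bullet actor that handles impact visuals and removes itself when it hits something.
; On Hit, it casts the struck actor to the player or enemy character and spawns a blood particle at the hit location for either.
; Other surfaces get a short-lived gunshot decal oriented to the hit normal plus two impact emitters.
; The graph applies no damage and contains no movement logic.
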(event `self.ReceiveHit`
  (params (MyComp :type "PrimitiveComponent Object Reference") (Other :type "Actor Object Reference") (OtherComp :type "PrimitiveComponent Object Reference") (bSelfMoved :type Boolean) (HitLocation :type "Vector Structure") (HitNormal :type "Vector Structure") (NormalImpulse :type "Vector Structure") (Hit :type "HitResult Structure (by ref)"))
  (set `self.HitLoc` HitLocation)
  (cast `/Game/Slealth/Blueprints/PlayerCharBP` Other
    (:`then`
      (`GameplayStatics.SpawnEmitterAtLocation` "/Game/Slealth/Particles/BloodParticle.BloodParticle" (`self.HitLoc`) :!label _label))
    (:`CastFailed`
      (cast `/Game/Slealth/Blueprints/EnemyCharBP` Other
        (:`then`
          (goto _label))
        (:`CastFailed`
          (`GameplayStatics.SpawnDecalAtLocation` "/Game/Slealth/MaterialTextures/GunShotMat.GunShotMat" (10.0 10.0 10.0) (`self.HitLoc`) (`KismetMathLibrary.MakeRotFromX` HitNormal) 10.0)
          (`GameplayStatics.SpawnEmitterAtLocation` "/Game/Slealth/Particles/BulletHitParticles.BulletHitParticles" (`self.HitLoc`))
          (`GameplayStatics.SpawnEmitterAtLocation` "/Game/Slealth/Particles/BulletHit2Particle.BulletHit2Particle" (`self.HitLoc`))))))
  (`self.K2_DestroyActor`))

(fn `UserConstructionScript`)