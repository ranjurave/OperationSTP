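; Stealth-game enemy character that shoots bullets, reacts to being hit and dies after a set number of bullet hits.
; Any hit alerts the AI by writing its own location, player visibility and chase status to the Blackboard.
; Bullet hits decrement a counter, playing a hit montage, or a death montage before destroying the actor.
; ShootPlayer spawns a bullet and muzzle effect with a brief firing flag, unless IsHit is set.
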(event `ResetDo`
  ;[1 1 1] Bullet hit
  (goto _label :!via `Reset`))

(event `self.ReceiveHit`
  (params (MyComp :type "PrimitiveComponent Object Reference") (Other :type "Actor Object Reference") (OtherComp :type "PrimitiveComponent Object Reference") (bSelfMoved :type Boolean) (HitLocation :type "Vector Structure") (HitNormal :type "Vector Structure") (NormalImpulse :type "Vector Structure") (Hit :type "HitResult Structure (by ref)"))
  ;[1 1 1] Bullet hit
  (`|ExecutionSequence`
    (:`then_0`
      ;[1 1 1] Alert enemy when hit by bullet
      (`BlackboardComponent.SetValueAsVector` (`AIBlueprintHelperLibrary.GetBlackboard` null) "TargetLocation" (`self.K2_GetActorLocation`))
      (`BlackboardComponent.SetValueAsBool` (`AIBlueprintHelperLibrary.GetBlackboard` null) "CanSeePlayer" true)
      (`BlackboardComponent.SetValueAsEnum` (`AIBlueprintHelperLibrary.GetBlackboard` null) "ChaseStatus" 2))
    (:`then_1`
      (cast `/Game/Slealth/Blueprints/Bullet` Other)
      (set `self.IsHit` true)
      (bind _result (`/Engine/EditorBlueprintResources/StandardMacros.DecrementInt` (`self.BulletHit`))
        (:`  `
          (set `self.BulletHit` _result)
          (if (> (`self.BulletHit`) 0)
            (`/Engine/EditorBlueprintResources/StandardMacros.DoOnce` false :!label _label
              (:`Completed`
                (`AnimInstance.Montage_Play` (`SkeletalMeshComponent.GetAnimInstance` (`self.Mesh`)) "/Game/Slealth/Animations/EnemyAnimation/HitEnemyMontage.HitEnemyMontage" 1.0 "MontageLength" 0.0 true)
                (set `self.IsHit` false)
                (`self.ResetDo`)))
            (else
              (`/Engine/EditorBlueprintResources/StandardMacros.DoOnce` false
                (:`Completed`
                  (`AnimInstance.Montage_Play` (`SkeletalMeshComponent.GetAnimInstance` (`self.Mesh`)) "/Game/Slealth/Animations/EnemyAnimation/DeathEnemyMontage.DeathEnemyMontage" 1.0 "MontageLength" 0.0 true)
                  (`KismetSystemLibrary.Delay` 1.6)
                  (`self.K2_DestroyActor`))))))))))

(event `ShootPlayer`
  (bind _returnvalue (`SceneComponent.K2_GetComponentRotation` (`self.CapsuleComponent`)))
  ;[1 1 1] Third person shooting
  (if (not (`self.IsHit`))
    (set `self.IsFiring` true)
    (`|SpawnActorFromClass` "/Game/Slealth/Blueprints/Bullet.Bullet_C" (`KismetMathLibrary.MakeTransform` (+ (`SceneComponent.K2_GetComponentLocation` (`self.SphereTPS`)) (`KismetMathLibrary.GreaterGreater_VectorRotator` (`self.GunOffsetTPS`) _returnvalue)) _returnvalue) "Undefined" "OverrideRootScale" null null)
    (`GameplayStatics.SpawnEmitterAtLocation` "/Game/Slealth/Particles/GunFireParticles.GunFireParticles" (`SceneComponent.K2_GetComponentLocation` (`self.SphereTPS`)) (struct) (0.2 0.2 0.2))
    (`KismetSystemLibrary.Delay` 0.2)
    (set `self.IsFiring` false)))

(fn `UserConstructionScript`)