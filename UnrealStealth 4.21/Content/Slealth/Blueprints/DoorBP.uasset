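; Level exit door for the stealth game that swings open for the player and loads another level.
; When the player character overlaps the actor, a timeline drives the yaw of the Scene component; nothing reverses it.
; When the player overlaps Box1, the door sets the StealthGI game instance's level number to one above the value cached at BeginPlay, then opens the level named by LevelName.
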(event `self.ReceiveBeginPlay`
  (bind _asstealth_gi (cast `/Game/Slealth/Blueprints/StealthGI` (`GameplayStatics.GetGameInstance`)))
  (bind _output_get (set `self.GI` _asstealth_gi))
  (set `self.LevelNumber` (`/Game/Slealth/Blueprints/StealthGI.LevelNumber` _output_get)))

(event `self.ReceiveActorBeginOverlap`
  (params (OtherActor :type "Actor Object Reference"))
  (cast `/Game/Slealth/Blueprints/PlayerCharBP` OtherActor)
  (bind (_direction _open) (`Timeline|DoorOpenTimeline`)
    (:`Update`
      (`SceneComponent.K2_SetRelativeRotation` (`self.Scene`) (`KismetMathLibrary.MakeRotator` 0.0 0.0 _open) false false))))

(event `self.Box1.OnComponentBeginOverlap`
  (params (OverlappedComponent :type "PrimitiveComponent Object Reference") (OtherActor :type "Actor Object Reference") (OtherComp :type "PrimitiveComponent Object Reference") (OtherBodyIndex :type Integer) (bFromSweep :type Boolean) (SweepResult :type "HitResult Structure (by ref)"))
  (cast `/Game/Slealth/Blueprints/PlayerCharBP` OtherActor)
  (set `/Game/Slealth/Blueprints/StealthGI.LevelNumber` (+ (`self.LevelNumber`) 1) (`self.GI`))
  (`GameplayStatics.OpenLevel` (`self.Level Name`)))

(fn `UserConstructionScript`)